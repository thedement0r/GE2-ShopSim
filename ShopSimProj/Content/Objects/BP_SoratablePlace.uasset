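; Storage place actor that displays items from the BP_Package the player is interacting with, one item type at a time.
; GiveAction accepts a matching name or an unset type, gated by an AmountPerStorage < CurrentAmount check (apparently inverted for a capacity limit).
; It finds the item's DT_Item row by name, spawns its actor class without collision or physics, snaps it to one of three slot components and increments the count.
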(event EventBeginPlay)

(event Collision|EventActorBeginOverlap
  (params (OtherActor :type Actor%20Object%20Reference)))

(event EventTick
  (params (DeltaSeconds :type Float%20%28single-precision%29)))

(event EventGiveAction
  (bind _currentamount (Variables|Default|GetCurrentAmount))
  (bind _scene (Variables|Default|GetScene))
  (bind _scene1 (Variables|Default|GetScene1))
  (bind _scene2 (Variables|Default|GetScene2))
  (bind _returnvalue (Utilities|Select :Index _currentamount :Option%200 _scene :Option%201 _scene1 :Option%202 _scene2))
  (bind _asbp_first_person_character (Utilities|Casting|CastToBP_FirstPersonCharacter (Game|GetPlayerCharacter 0)))
  (bind _asbp_package (Utilities|Casting|CastToBP_Package (Variables|/Game/FirstPerson/Blueprints/BP_FirstPersonCharacter.BP_FirstPersonCharacter_C|GetInteractableActor _asbp_first_person_character)))
  (if (and (< (Variables|Default|GetAmountPerStorage) (Variables|Default|GetCurrentAmount)) (or (Utilities|Text|TextIsEmpty (.Name (Utilities|Struct|BreakS_Item (Variables|Default|GetStoragedItemInfo)))) (Utilities|Enum|Equal(Enum) (.Name (Utilities|Struct|BreakS_Item (Variables|/Game/Objects/BP_Package.BP_Package_C|GetItemInfo _asbp_package))) (.Name (Utilities|Struct|BreakS_Item (Variables|Default|GetStoragedItemInfo))))))
    (bind _output_get (Variables|Default|SetStoragedItemInfo (Variables|/Game/Objects/BP_Package.BP_Package_C|GetItemInfo _asbp_package)))
    (bind _outrownames (DataTable|GetDataTableRowNames 0))
    (bind _array_element (Utilities|Array|ForEachLoopwithBreak _outrownames)
      (:LoopBody
        (bind _returnvalue_2 (Utilities|GetDataTableRow "/Game/Objects/DT_Item.DT_Item" _array_element)
          (:then
            (if (Utilities|Enum|Equal(Enum) (.Name (Utilities|Struct|BreakS_Item _returnvalue_2)) (.Name (Utilities|Struct|BreakS_Item _output_get)))
              (bind _returnvalue_3 (Game|SpawnActorfromClass (.ActorClass (Utilities|Struct|BreakS_Item _returnvalue_2)) (Math|Transform|MakeTransform (Transformation|GetWorldLocation _returnvalue)) "Undefined" "MultiplyWithRoot" 0 (Utilities|Struct|MakeDataTableRowHandle "/Game/Objects/DT_Item.DT_Item" _array_element) 0))
              (Collision|SetCollisionEnabled (Variables|/Game/Objects/BP_Item.BP_Item_C|GetItem _returnvalue_3) "NoCollision")
              (Transformation|AttachComponentToComponent _returnvalue_3 _returnvalue "None" "SnapToTarget" "SnapToTarget" "SnapToTarget" true)
              (Physics|SetSimulatePhysics (Variables|/Game/Objects/BP_Item.BP_Item_C|GetItem _returnvalue_3) false)
              (Math|Integer|IncrementInt (Variables|Default|GetCurrentAmount)))))))))

(fn ConstructionScript)

(fn StartGrabbing
  (return false))

(fn StopGrabbing
  (return false))