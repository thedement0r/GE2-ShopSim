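; BP_Item is a world item that can be highlighted and, when CanGrab is set, grabbed by the player.
; On BeginPlay a grabbable item enables physics simulation on its Item component.
; StartGrabbing and StopGrabbing grab and release it through the PhysicsHandleComponent on the first player character, returning whether the item allows grabbing.
; SetOverlay toggles an outline overlay material on the mesh for highlighting.
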(event EventSetOverlay
  (params (EnableOverlay :type Boolean))
  ;[0.15 0.15 0.15 0.5] Set item overlay
  (Rendering|Material|SetOverlayMaterial (Variables|Default|GetItem) (select EnableOverlay "/Game/Objects/M_Outline.M_Outline" 0) :!class /Script/Engine.MeshComponent))

(event EventBeginPlay
  (if (Variables|Default|GetcanGrab)
    (Physics|SetSimulatePhysics (Variables|Default|GetItem) true)))

(fn ConstructionScript)

(fn StartGrabbing
  (bind _item (Variables|Default|GetItem))
  (if (Variables|Default|GetcanGrab)
    (Physics|Components|PhysicsHandle|GrabComponentatLocationwithRotation (Actor|GetComponentbyClass (Game|GetPlayerCharacter 0) "/Script/Engine.PhysicsHandleComponent") _item "None" (Transformation|GetWorldLocation _item) "0, 0, 0")
    (return true)
    (else
      (return false))))

(fn StopGrabbing
  (if (Variables|Default|GetcanGrab)
    (Physics|Components|PhysicsHandle|ReleaseComponent (Actor|GetComponentbyClass (Game|GetPlayerCharacter 0) "/Script/Engine.PhysicsHandleComponent"))
    (return true)
    (else
      (return false))))