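; BP_Package is a package actor that the first-person player can interact with and pick up.
; Interaction copies the package's ItemRowName to the character's HeldItemID, but only if HoldingItem is already true.
; PickUpPackage disables collision, attaches the package to the first-person camera and sets a fixed relative offset and rotation.
; A DT_Item row lookup with debug prints is left unconnected and never runs.
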(event Custom|PickUpPackage
  (Collision|SetActorEnableCollision false)
  (bind _asbp_first_person_character (Utilities|Casting|CastToBP_FirstPersonCharacter (Game|GetPlayerCharacter 0)))
  (Transformation|AttachComponentToComponent (Variables|/Game/FirstPerson/Blueprints/BP_FirstPersonCharacter.BP_FirstPersonCharacter_C|GetFirstPersonCamera _asbp_first_person_character) "None" "SnapToTarget" "SnapToTarget" "KeepWorld" false)
  (Transformation|SetActorRelativeLocation "100.000000,0.000000,-40.000000")
  (Transformation|SetActorRelativeRotation "0, 0, 0"))

(event EventBeginPlay
  ;[0.15 0.15 0.15 0.5] currently disable
)

(event Collision|EventActorBeginOverlap
  (params (OtherActor :type Actor%20Object%20Reference)))

(event EventTick
  (params (DeltaSeconds :type Float%20%28single-precision%29)))

(event EventInteraction
  (bind _asbp_first_person_character (Utilities|Casting|CastToBP_FirstPersonCharacter (Game|GetPlayerCharacter 0)))
  (if (Variables|/Game/FirstPerson/Blueprints/BP_FirstPersonCharacter.BP_FirstPersonCharacter_C|GetbHoldingItem _asbp_first_person_character)
    (Variables|/Game/FirstPerson/Blueprints/BP_FirstPersonCharacter.BP_FirstPersonCharacter_C|SetHeldItemID _asbp_first_person_character (Variables|Default|GetItemRowName))
    (Variables|/Game/FirstPerson/Blueprints/BP_FirstPersonCharacter.BP_FirstPersonCharacter_C|SetbHoldingItem _asbp_first_person_character true)))

(fn ConstructionScript)