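; BP_Cube is a pickup cube actor that shows a label while another actor overlaps it.
; Overlap begin and end events toggle the Label component's visibility.
; Interact prints a pickup message, triggers DestroyItem and returns the SMCube static mesh to the caller.
; DestroyItem runs as an event so it can wait briefly before destroying the actor.
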(event Custom|Destroy%20Item
  (Utilities|FlowControl|Delay 0.2)
  (Actor|DestroyActor))

(event Collision|EventActorBeginOverlap
  (params (OtherActor :type Actor%20Object%20Reference))
  (Rendering|SetVisibility (Variables|Default|GetLabel%20) true false))

(event Collision|EventActorEndOverlap
  (params (OtherActor :type Actor%20Object%20Reference))
  (Rendering|SetVisibility (Variables|Default|GetLabel%20) false false))

(fn ConstructionScript)

(fn Interact
  (Development|PrintString "Picked")
  (CallFunction|DestroyItem)
  (return (Variables|/Script/Engine.StaticMeshComponent|GetStaticMesh (Variables|Default|GetSM_Cube))))