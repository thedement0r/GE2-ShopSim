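; BP_Shelfitem is a store shelf that holds up to six item meshes and automatically sells them for money and skill points.
; PlacePackage adds a mesh from the package's item data at the next slot, specially scales Rice, and destroys the package.
; A looping timer, scaled by the player's interval modifier at BeginPlay, runs SellRandomItem.
; Despite its name, that event removes the first stored item without shifting the others, then credits the player.
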(event Custom|PlacePackage
  (params (PackageRef :type BP%20Package%20Object%20Reference))
  (bind _itemdata (Variables|/Game/Objects/BP_Package.BP_Package_C|GetItemData PackageRef))
  (bind (_name _description _price _thumbail _actorclass _unitamount _storagetype _type _itemmesh) (Utilities|Struct|BreakS_Item _itemdata))
  (if (< (Variables|Default|GetNextSlotIndex) (Utilities|Array|Length (Variables|Default|GetSpawnPoints)))
    (Utilities|IsValid PackageRef
      (:Is%20Valid
        (bind _returnvalue (AddComponent|AddStaticMeshComponent false))
        (if (Utilities|Enum|Equal(Enum) _name (Variables|Default|Getrice))
          (Transformation|SetRelativeScale3D _returnvalue "0.020000,0.020000,0.020000"))
        (bind _output_get (Variables|Default|SetNewMesh _returnvalue))
        (Components|StaticMesh|SetStaticMesh _output_get _itemmesh)
        (Transformation|AttachComponentToComponent _output_get (Utilities|Array|Get(acopy) (Variables|Default|GetSpawnPoints) (Variables|Default|GetNextSlotIndex)) "None" "KeepRelative" "KeepRelative" "KeepRelative" false)
        (bind _result (Math|Integer|IncrementInt (Variables|Default|GetNextSlotIndex))
          (:%20%20
            (Variables|Default|SetNextSlotIndex _result)
            (Utilities|Array|Add (Variables|Default|GetStoredItems) _output_get)
            (Development|PrintString "destrooy ")
            (Actor|DestroyActor PackageRef)))))
    (else
      (Development|PrintString "Full shelf"))))

(event Custom|SellRandomItem
  (if (> (Utilities|Array|Length (Variables|Default|GetStoredItems)) 0)
    (Components|DestroyComponent (Utilities|Array|Get(acopy) (Variables|Default|GetStoredItems)))
    (Utilities|Array|RemoveIndex (Variables|Default|GetStoredItems))
    (Variables|Default|SetNextSlotIndex (Utilities|Array|Length (Variables|Default|GetStoredItems)))
    (bind _asbp_first_person_character (Utilities|Casting|CastToBP_FirstPersonCharacter (Game|GetPlayerCharacter 0)))
    (Variables|/Game/FirstPerson/Blueprints/BP_FirstPersonCharacter.BP_FirstPersonCharacter_C|SetCurrentMoney _asbp_first_person_character (+ (Variables|/Game/FirstPerson/Blueprints/BP_FirstPersonCharacter.BP_FirstPersonCharacter_C|GetCurrentMoney _asbp_first_person_character) (* (Variables|Default|GetMoneyPerItem) (Variables|/Game/FirstPerson/Blueprints/BP_FirstPersonCharacter.BP_FirstPersonCharacter_C|GetSellMoneyModifier _asbp_first_person_character))))
    (Default|UpdateMoney _asbp_first_person_character 0.0)
    (Variables|/Game/FirstPerson/Blueprints/BP_FirstPersonCharacter.BP_FirstPersonCharacter_C|Setpoints _asbp_first_person_character (+ (Variables|/Game/FirstPerson/Blueprints/BP_FirstPersonCharacter.BP_FirstPersonCharacter_C|GetSkillPointsPerSale _asbp_first_person_character) (Variables|/Game/FirstPerson/Blueprints/BP_FirstPersonCharacter.BP_FirstPersonCharacter_C|Getpoints _asbp_first_person_character)))))

(event EventBeginPlay
  (Utilities|Array|Clear (Variables|Default|GetSpawnPoints))
  (Utilities|Array|Add (Variables|Default|GetSpawnPoints) (Variables|Default|GetChildActor))
  (Utilities|Array|Add (Variables|Default|GetSpawnPoints) (Variables|Default|GetChildActor1))
  (Utilities|Array|Add (Variables|Default|GetSpawnPoints) (Variables|Default|GetChildActor2))
  (Utilities|Array|Add (Variables|Default|GetSpawnPoints) (Variables|Default|GetChildActor3))
  (Utilities|Array|Add (Variables|Default|GetSpawnPoints) (Variables|Default|GetChildActor4))
  (Utilities|Array|Add (Variables|Default|GetSpawnPoints) (Variables|Default|GetChildActor5))
  (bind _asbp_first_person_character (Utilities|Casting|CastToBP_FirstPersonCharacter (Game|GetPlayerCharacter 0)))
  (Utilities|Time|SetTimerbyEvent (delegate Custom|SellRandomItem) (* (Variables|Default|GetSellInterval) (Variables|/Game/FirstPerson/Blueprints/BP_FirstPersonCharacter.BP_FirstPersonCharacter_C|GetSellIntervalModifier _asbp_first_person_character)) true))

(event Collision|EventActorBeginOverlap
  (params (OtherActor :type Actor%20Object%20Reference)))

(event EventTick
  (params (DeltaSeconds :type Float%20%28single-precision%29)))

(fn ConstructionScript
  (|CallParentFunction))