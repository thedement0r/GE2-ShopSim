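; BP_Bounds is an out-of-bounds volume that restarts the level if the player stays inside it.
; When BP_FirstPersonCharacter enters BoundsTrigger, it sets OutOfBounds, shows the WB_OUT widget and starts a three-second delay.
; Leaving clears the flag and removes the widget; the delay keeps running, but the Restartlevel console command fires only if the flag is set when it ends.
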(event OnComponentBeginOverlap(BoundsTrigger)
  (params (OverlappedComponent :type Primitive%20Component%20Object%20Reference) (OtherActor :type Actor%20Object%20Reference) (OtherComp :type Primitive%20Component%20Object%20Reference) (OtherBodyIndex :type Integer) (bFromSweep :type Boolean) (SweepResult :type Hit%20Result%20Structure%20%28by%20ref%29))
  (Utilities|Casting|CastToBP_FirstPersonCharacter OtherActor)
  (Variables|Default|SetoutOfBounds true)
  (bind _returnvalue (UserInterface|CreateWidget "/Game/WB_OUT.WB_OUT_C"))
  (bind _output_get (Variables|Default|SetOut_Widget _returnvalue))
  (UserInterface|Viewport|AddtoViewport _output_get 0)
  (Utilities|FlowControl|Delay 3.0)
  (if (Variables|Default|GetoutOfBounds)
    (Development|ExecuteConsoleCommand "Restartlevel" 0)))

(event OnComponentEndOverlap(BoundsTrigger)
  (params (OverlappedComponent :type Primitive%20Component%20Object%20Reference) (OtherActor :type Actor%20Object%20Reference) (OtherComp :type Primitive%20Component%20Object%20Reference) (OtherBodyIndex :type Integer))
  (Utilities|Casting|CastToBP_FirstPersonCharacter OtherActor)
  (Variables|Default|SetoutOfBounds false)
  (bind _out_widget (Variables|Default|GetOut_Widget)
    (:then
      (Widget|RemovefromParent _out_widget)
      (Variables|Default|SetOut_Widget 0))
    (:else)))

(event EventBeginPlay)

(event Collision|EventActorBeginOverlap
  (params (OtherActor :type Actor%20Object%20Reference)))

(event EventTick
  (params (DeltaSeconds :type Float%20%28single-precision%29)))

(fn ConstructionScript)